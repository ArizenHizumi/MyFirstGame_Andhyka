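; BP_CobaArray is a tutorial Blueprint that tries out basic array operations on ArrayName.
; On BeginPlay it adds one name, removes another by value, then prints each element and the resulting array length.
; A remove-by-index node is left unconnected and never runs, and the construction script is empty.
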(event `self.ReceiveBeginPlay`
  (bind _arrayname (`self.ArrayName`))
  (`KismetArrayLibrary.Array_Add` (`self.ArrayName`) "Johan")
  (`KismetArrayLibrary.Array_RemoveItem` _arrayname "Fadhli")
  (for _array_element (`self.ArrayName`)
    (`KismetSystemLibrary.PrintString` _array_element))
  (`KismetSystemLibrary.PrintString` (`KismetStringLibrary.Conv_IntToString` (`KismetArrayLibrary.Array_Length` _arrayname))))

(fn `UserConstructionScript`)