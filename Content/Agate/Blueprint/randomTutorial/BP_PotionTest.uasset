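; BP_PotionTest is a tutorial Blueprint for practising functions and flow control around a potion-based Health system.
; DrinkPotion raises Health by a fixed amount and prints it, SistemTambahHP adds a passed-in amount, and Pernomoran returns the sum of two numbers.
; The event graph holds loop, branch and FlipFlop experiments calling these helpers, but no event drives them, so none run.
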(event `Key|RightShift`
  (params (Key :type "Key Structure")))

(event `Key|Tab`
  (params (Key :type "Key Structure")))

(event `Key|CapsLock`
  (params (Key :type "Key Structure")))

(event `Key|LeftShift`
  (params (Key :type "Key Structure")))

(fn `Drink Potion`
  (`KismetSystemLibrary.PrintString` "Drink Complete")
  (set `self.Health` (+ (`self.Health`) 20))
  (`KismetSystemLibrary.PrintString` (`KismetStringLibrary.Conv_IntToString` (`self.Health`))))

(fn `Pernomoran?`
  (params (`Nomor 1` :type Integer) (`Nomor 2` :type Integer))
  (returns (Hasil :type Integer))
  (return (+ `Nomor 1` `Nomor 2`)))

(fn `SistemTambahHP`
  (params (DynamicHealth :type Integer))
  (set `self.Health` (+ (`self.Health`) DynamicHealth)))

(fn `UserConstructionScript`)