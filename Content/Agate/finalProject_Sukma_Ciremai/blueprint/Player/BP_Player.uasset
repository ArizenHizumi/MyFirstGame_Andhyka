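; Player character for a third-person shooter, handling Enhanced Input movement, weapons, health, death and pause.
; An overlap detector finds BP_Weapon pickups, whose data drives holstered/armed mesh swaps, fire rate, range and ammo limits.
; Aiming shows a crosshair and shortens the spring arm by timeline, enabling DoOnce-throttled line-trace shots from the muzzle that damage BP_Enemy.
; Damage updates the HUD bar and triggers the lose screen; ammo prints as debug text.
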(event `self.ReceiveBeginPlay`
  (bind _asplayer_controller (cast `PlayerController` (`self.GetController`)))
  (`EnhancedInputSubsystemInterface.AddMappingContext` (pcsubsystem `EnhancedInputLocalPlayerSubsystem` _asplayer_controller) "/Game/Agate/finalProject_Sukma_Ciremai/blueprint/Input/IMC_Default.IMC_Default" 0 (struct))
  (set `CharacterMovementComponent.MaxWalkSpeed` (`self.WalkingSpeed`) (`self.CharacterMovement`))
  (set `self.Health` (`self.MaxHealth`))
  (bind _returnvalue (`|CreateWidget` "/Game/Agate/finalProject_Sukma_Ciremai/blueprint/User_Interface/WBP_HUD.WBP_HUD_C"))
  (`UserWidget.AddToViewport` _returnvalue 0)
  (set `self.WBP Health Bar Player` (`/Game/Agate/finalProject_Sukma_Ciremai/blueprint/User_Interface/WBP_HUD.WBP_HealthBarPlayer` _returnvalue))
  (`/Game/Agate/finalProject_Sukma_Ciremai/blueprint/User_Interface/WBP_HealthPlayer.SetHealthBarValue` (`self.WBP Health Bar Player`) (`KismetMathLibrary.Conv_IntToDouble` (`self.Health`)) (`KismetMathLibrary.Conv_IntToDouble` (`self.MaxHealth`))))

(event `EnhancedInput|/Game/Agate/finalProject_Sukma_Ciremai/blueprint/Input/IA_Move`
  (params (ActionValue :type "Vector2D Structure") (ElapsedSeconds :type "Float (double-precision)") (TriggeredSeconds :type "Float (double-precision)") (InputAction :type "InputAction Object Reference" :default "/Game/Agate/finalProject_Sukma_Ciremai/blueprint/Input/IA_Move.IA_Move"))
  (bind (_returnvalue_roll _returnvalue_pitch _returnvalue_yaw) (`KismetMathLibrary.BreakRotator` (`self.GetControlRotation`)))
  (:`Triggered`
    (`self.AddMovementInput` (`KismetMathLibrary.GetRightVector` (`self.GetControlRotation`)) ActionValue_X)
    (`self.AddMovementInput` (`KismetMathLibrary.GetForwardVector` (`KismetMathLibrary.MakeRotator` _returnvalue_roll 0.0 _returnvalue_yaw)) ActionValue_Y)))

(event `EnhancedInput|/Game/Agate/finalProject_Sukma_Ciremai/blueprint/Input/IA_Look`
  (params (ActionValue :type "Vector2D Structure") (ElapsedSeconds :type "Float (double-precision)") (TriggeredSeconds :type "Float (double-precision)") (InputAction :type "InputAction Object Reference" :default "/Game/Agate/finalProject_Sukma_Ciremai/blueprint/Input/IA_Look.IA_Look"))
  (:`Triggered`
    (`self.AddControllerYawInput` ActionValue_X)
    (`self.AddControllerPitchInput` ActionValue_Y)))

(event `EnhancedInput|/Game/Agate/finalProject_Sukma_Ciremai/blueprint/Input/IA_Sprint`
  (params (ActionValue :type Boolean) (ElapsedSeconds :type "Float (double-precision)") (TriggeredSeconds :type "Float (double-precision)") (InputAction :type "InputAction Object Reference" :default "/Game/Agate/finalProject_Sukma_Ciremai/blueprint/Input/IA_Sprint.IA_Sprint"))
  (bind _charactermovement (`self.CharacterMovement`))
  (:`Started`
    (set `CharacterMovementComponent.MaxWalkSpeed` (`self.SprintSpeed`) _charactermovement))
  (:`Completed`
    (set `CharacterMovementComponent.MaxWalkSpeed` (`self.WalkingSpeed`) _charactermovement)))

(event `self.PickupDetector.OnComponentBeginOverlap`
  (params (OverlappedComponent :type "PrimitiveComponent Object Reference") (OtherActor :type "Actor Object Reference") (OtherComp :type "PrimitiveComponent Object Reference") (OtherBodyIndex :type Integer) (bFromSweep :type Boolean) (SweepResult :type "HitResult Structure (by ref)"))
  (bind _asbp_weapon (cast `/Game/Agate/finalProject_Sukma_Ciremai/blueprint/Weapon/BP_Weapon` OtherActor))
  (set `self.DetectedWeapon` _asbp_weapon))

(event `self.PickupDetector.OnComponentEndOverlap`
  (params (OverlappedComponent :type "PrimitiveComponent Object Reference") (OtherActor :type "Actor Object Reference") (OtherComp :type "PrimitiveComponent Object Reference") (OtherBodyIndex :type Integer))
  (set `self.DetectedWeapon` null))

(event `EnhancedInput|/Game/Agate/finalProject_Sukma_Ciremai/blueprint/Input/IA_Pickup`
  (params (ActionValue :type Boolean) (ElapsedSeconds :type "Float (double-precision)") (TriggeredSeconds :type "Float (double-precision)") (InputAction :type "InputAction Object Reference" :default "/Game/Agate/finalProject_Sukma_Ciremai/blueprint/Input/IA_Pickup.IA_Pickup"))
  (:`Started`
    (`/Engine/EditorBlueprintResources/StandardMacros.IsValid` (`self.DetectedWeapon`)
      (:`Is Valid`
        (set `self.Weapon` (`/Game/Agate/finalProject_Sukma_Ciremai/blueprint/Weapon/BP_Weapon.WeaponData` (`self.DetectedWeapon`)))
        (`self.K2_DestroyActor` (`self.DetectedWeapon`))
        (set `self.DetectedWeapon` null)
        (`SkeletalMeshComponent.SetSkeletalMeshAsset` (`self.HolsterWeaponMesh`) (`/Game/Agate/finalProject_Sukma_Ciremai/blueprint/Weapon/Data/BP_WeaponData.Mesh` (`self.Weapon`)))))))

(event `EnhancedInput|/Game/Agate/finalProject_Sukma_Ciremai/blueprint/Input/IA_Holster`
  (params (ActionValue :type Boolean) (ElapsedSeconds :type "Float (double-precision)") (TriggeredSeconds :type "Float (double-precision)") (InputAction :type "InputAction Object Reference" :default "/Game/Agate/finalProject_Sukma_Ciremai/blueprint/Input/IA_Holster.IA_Holster"))
  (:`Started`
    (`/Engine/EditorBlueprintResources/StandardMacros.IsValid` (`self.Weapon`)
      (:`Is Valid`
        (if (`self.IsWeaponHolster`)
          (set `self.IsWeaponHolster` false)
          (`SkeletalMeshComponent.SetSkeletalMeshAsset` (`self.HolsterWeaponMesh`) null)
          (`SkeletalMeshComponent.SetSkeletalMeshAsset` (`self.ArmedWeaponMesh`) (`/Game/Agate/finalProject_Sukma_Ciremai/blueprint/Weapon/Data/BP_WeaponData.Mesh` (`self.Weapon`)))
          (else
            (set `self.IsWeaponHolster` true)
            (`SkeletalMeshComponent.SetSkeletalMeshAsset` (`self.HolsterWeaponMesh`) (`/Game/Agate/finalProject_Sukma_Ciremai/blueprint/Weapon/Data/BP_WeaponData.Mesh` (`self.Weapon`)))
            (`SkeletalMeshComponent.SetSkeletalMeshAsset` (`self.ArmedWeaponMesh`) null)))))))

(event `EnhancedInput|/Game/Agate/finalProject_Sukma_Ciremai/blueprint/Input/IA_Aim`
  (params (ActionValue :type Boolean) (ElapsedSeconds :type "Float (double-precision)") (TriggeredSeconds :type "Float (double-precision)") (InputAction :type "InputAction Object Reference" :default "/Game/Agate/finalProject_Sukma_Ciremai/blueprint/Input/IA_Aim.IA_Aim"))
  (bind _charactermovement (`self.CharacterMovement`))
  (bind _charactermovement_2 (`self.CharacterMovement`))
  (:`Started`
    (if (and (`KismetSystemLibrary.IsValid` (`self.Weapon`)) (not (`self.IsWeaponHolster`)))
      (bind _returnvalue (`|CreateWidget` "/Game/Agate/finalProject_Sukma_Ciremai/blueprint/User_Interface/WBP_Crosshair.WBP_Crosshair_C" (`GameplayStatics.GetPlayerController` 0)))
      (bind _output_get (set `self.isCrosshairOn?` _returnvalue))
      (`UserWidget.AddToViewport` _output_get 0)
      (set `self.IsAiming` true)
      (set `CharacterMovementComponent.bUseControllerDesiredRotation` true _charactermovement)
      (set `CharacterMovementComponent.bOrientRotationToMovement` false _charactermovement)
      (bind (_direction _alpha) (`Timeline|AimTransition` :!label _label)
        (:`Update`
          (set `SpringArmComponent.TargetArmLength` (`KismetMathLibrary.Lerp` 150.0 70.0 _alpha) (`self.SpringArm`))))))
  (:`Completed`
    (`Widget.RemoveFromParent` (`self.isCrosshairOn?`))
    (set `self.IsAiming` false)
    (set `CharacterMovementComponent.bUseControllerDesiredRotation` false _charactermovement_2)
    (set `CharacterMovementComponent.bOrientRotationToMovement` true _charactermovement_2)
    (goto _label :!via `Reverse`)))

(event `EnhancedInput|/Game/Agate/finalProject_Sukma_Ciremai/blueprint/Input/IA_Shoot`
  (params (ActionValue :type Boolean) (ElapsedSeconds :type "Float (double-precision)") (TriggeredSeconds :type "Float (double-precision)") (InputAction :type "InputAction Object Reference" :default "/Game/Agate/finalProject_Sukma_Ciremai/blueprint/Input/IA_Shoot.IA_Shoot"))
  (bind _returnvalue (`SceneComponent.GetSocketLocation` (`self.ArmedWeaponMesh`) "MuzzleSocket"))
  (:`Triggered`
    (if (and (`self.IsAiming`) (> (`self.MagazineAmmunition`) 0))
      (`|ExecutionSequence`
        (:`then_0`
          (`/Engine/EditorBlueprintResources/StandardMacros.DoOnce` false :!label _label_2
            (:`Completed`
              (`|PlayMontage` (`self.Mesh`) "/Game/Agate/Custom_Asset/Player/Josh_mixamo/Animation/AM_Shoot.AM_Shoot"
                (:`then`
                  (`GameplayStatics.SpawnEmitterAttached` "/Game/InfinityBladeEffects/Effects/FX_Monsters/FX_Monster_Gruntling/Master/P_BackPack_MuzzleFlash.P_BackPack_MuzzleFlash" (`self.ArmedWeaponMesh`) "MuzzleSocket" (0.0 0.0 0.0) (struct :`Pitch` 170.0) (150.0 150.0 150.0))
                  (`GameplayStatics.PlaySoundAtLocation` "/Game/Agate/Custom_Asset/Audio/shoot.shoot" _returnvalue (struct) 1.0 1.0 0.0 null null null null)
                  (bind _outhit (`KismetSystemLibrary.LineTraceSingle` :`Start` _returnvalue :`End` (+ _returnvalue (* (`KismetMathLibrary.GetForwardVector` (`SceneComponent.K2_GetComponentRotation` (`self.Camera`))) (`/Game/Agate/finalProject_Sukma_Ciremai/blueprint/Weapon/Data/BP_WeaponData.FireDistance` (`self.Weapon`)))) :`TraceChannel` "TraceTypeQuery1" :`TraceColor` (struct :`R` 1.0 :`G` 1.0 :`B` 1.0 :`A` 1.0) :`DrawTime` 2.0))
                  (set `self.MagazineAmmunition` (- (`self.MagazineAmmunition`) 1))
                  (`GameplayStatics.SpawnEmitterAtLocation` "/Game/InfinityBladeEffects/Effects/FX_Monsters/FX_Monster_GolemBot/Notifies/P_SparkBurst.P_SparkBurst" (`.Location` (`GameplayStatics.BreakHitResult` _outhit)))
                  (bind _asbp_enemy (cast `/Game/Agate/finalProject_Sukma_Ciremai/blueprint/Enemy/BP_Enemy` (`.HitActor` (`GameplayStatics.BreakHitResult` _outhit))))
                  (`GameplayStatics.ApplyDamage` _asbp_enemy 35.0))))))
        (:`then_1`
          (`KismetSystemLibrary.Delay` (`/Game/Agate/finalProject_Sukma_Ciremai/blueprint/Weapon/Data/BP_WeaponData.FireRate` (`self.Weapon`)))
          (goto _label_2 :!via `Reset`))))))

(event `EnhancedInput|/Game/Agate/finalProject_Sukma_Ciremai/blueprint/Input/IA_Reload`
  (params (ActionValue :type Boolean) (ElapsedSeconds :type "Float (double-precision)") (TriggeredSeconds :type "Float (double-precision)") (InputAction :type "InputAction Object Reference" :default "/Game/Agate/finalProject_Sukma_Ciremai/blueprint/Input/IA_Reload.IA_Reload"))
  (bind _returnvalue (- (`/Game/Agate/finalProject_Sukma_Ciremai/blueprint/Weapon/Data/BP_WeaponData.MaxMagazine` (`self.Weapon`)) (`self.MagazineAmmunition`)))
  (:`Started`
    (if (and (< (`self.MagazineAmmunition`) (`/Game/Agate/finalProject_Sukma_Ciremai/blueprint/Weapon/Data/BP_WeaponData.MaxMagazine` (`self.Weapon`))) (> (`self.TotalAmmunition`) 0))
      (`|PlayMontage` (`self.Mesh`) "/Game/Agate/Custom_Asset/Player/Josh_mixamo/Animation/Hasil_Retarget/AM_Reload.AM_Reload"
        (:`then`
          (`GameplayStatics.PlaySoundAtLocation` "/Game/Agate/Custom_Asset/Audio/reload.reload" (`SceneComponent.GetSocketLocation` (`self.ArmedWeaponMesh`) "MuzzleSocket") (struct) 1.0 1.0 0.0 null null null null))
        (:`OnCompleted`
          (if (>= (`self.TotalAmmunition`) _returnvalue)
            (set `self.TotalAmmunition` (- (`self.TotalAmmunition`) _returnvalue))
            (set `self.MagazineAmmunition` (+ (`self.MagazineAmmunition`) _returnvalue))
            (else
              (set `self.MagazineAmmunition` (+ (`self.MagazineAmmunition`) (`self.TotalAmmunition`)))
              (set `self.TotalAmmunition` (- (`self.TotalAmmunition`) (`self.TotalAmmunition`))))))))))

(event `self.ReceiveAnyDamage`
  (params (Damage :type "Float (single-precision)") (DamageType :type "DamageType Object Reference") (InstigatedBy :type "Controller Object Reference") (DamageCauser :type "Actor Object Reference"))
  (bind _returnvalue (`GameplayStatics.GetPlayerController` 0))
  (if (not (`self.IsDeath`))
    (set `self.Health` (- (`self.Health`) Damage))
    (cast `PlayerController` (`self.GetController`))
    (`/Game/Agate/finalProject_Sukma_Ciremai/blueprint/User_Interface/WBP_HealthPlayer.SetHealthBarValue` (`self.WBP Health Bar Player`) (`KismetMathLibrary.Conv_IntToDouble` (`self.Health`)) (`KismetMathLibrary.Conv_IntToDouble` (`self.MaxHealth`)))
    (if (<= (`self.Health`) 0)
      (set `self.IsDeath` true)
      (bind _returnvalue_2 (`|CreateWidget` "/Game/Agate/finalProject_Sukma_Ciremai/blueprint/User_Interface/WBP_GameLose.WBP_GameLose_C"))
      (`UserWidget.AddToViewport` _returnvalue_2 0)
      (set `PlayerController.bShowMouseCursor` true _returnvalue)
      (`WidgetBlueprintLibrary.SetInputMode_UIOnlyEx` _returnvalue null)
      (`|PlayMontage` (`self.Mesh`) "/Game/Agate/Custom_Asset/Player/Josh_mixamo/Animation/AM_Dying.AM_Dying"))))

(event `EnhancedInput|/Game/Agate/finalProject_Sukma_Ciremai/blueprint/Input/IA_Pause`
  (params (ActionValue :type Boolean) (ElapsedSeconds :type "Float (double-precision)") (TriggeredSeconds :type "Float (double-precision)") (InputAction :type "InputAction Object Reference" :default "/Game/Agate/finalProject_Sukma_Ciremai/blueprint/Input/IA_Pause.IA_Pause"))
  (bind _returnvalue (`GameplayStatics.GetPlayerController` 0))
  (:`Started`
    (if (not (`self.isPauseOpened?`))
      (set `self.isPauseOpened?` true)
      (bind _returnvalue_2 (`|CreateWidget` "/Game/Agate/finalProject_Sukma_Ciremai/blueprint/User_Interface/WBP_GamePause.WBP_GamePause_C" _returnvalue))
      (bind _output_get (set `self.PauseMenuWidget` _returnvalue_2))
      (`UserWidget.AddToViewport` _output_get 0)
      (`WidgetBlueprintLibrary.SetInputMode_GameAndUIEx` _returnvalue (`self.PauseMenuWidget`))
      (set `PlayerController.bShowMouseCursor` true (`GameplayStatics.GetPlayerController` 0))
      (`GameplayStatics.SetGamePaused` true)
      (else
        (set `self.isPauseOpened?` false)
        (`Widget.RemoveFromParent` (`self.PauseMenuWidget`))
        (`GameplayStatics.SetGamePaused` false)
        (`WidgetBlueprintLibrary.SetInputMode_GameOnly` _returnvalue)
        (set `PlayerController.bShowMouseCursor` false (`GameplayStatics.GetPlayerController` 0))))))

(event `self.ReceiveTick`
  (params (DeltaSeconds :type "Float (single-precision)"))
  (`KismetSystemLibrary.PrintString` (`KismetStringLibrary.Concat_StrStr` (`KismetStringLibrary.Conv_IntToString` (`self.MagazineAmmunition`)) "/" (`KismetStringLibrary.Conv_IntToString` (`self.TotalAmmunition`))) true true (struct :`G` 0.66 :`B` 1.0 :`A` 1.0) 0.01))

(fn `AddAmmunition`
  (params (AmmunitionToAdd :type Integer))
  (set `self.TotalAmmunition` (+ (`self.TotalAmmunition`) AmmunitionToAdd))
  (if (> (`self.TotalAmmunition`) (`/Game/Agate/finalProject_Sukma_Ciremai/blueprint/Weapon/Data/BP_WeaponData.MaxAmmunition` (`self.Weapon`)))
    (set `self.TotalAmmunition` (`/Game/Agate/finalProject_Sukma_Ciremai/blueprint/Weapon/Data/BP_WeaponData.MaxAmmunition` (`self.Weapon`)))))

(fn `AddHealth`
  (params (HealthToAdd :type Integer))
  (set `self.Health` (+ (`self.Health`) HealthToAdd))
  (if (> (`self.Health`) (`self.MaxHealth`))
    (set `self.Health` (`self.MaxHealth`))
    (`/Game/Agate/finalProject_Sukma_Ciremai/blueprint/User_Interface/WBP_HealthPlayer.SetHealthBarValue` (`self.WBP Health Bar Player`) (`KismetMathLibrary.Conv_IntToDouble` (`self.Health`)) (`KismetMathLibrary.Conv_IntToDouble` (`self.MaxHealth`)))))

(fn `UserConstructionScript`)