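; BP_Enemy is an AI enemy pawn that takes damage, ragdolls at zero health, drops BP_Ammunition and is destroyed after a short delay.
; PawnSensing flags a seen BP_Player in the AI controller's Blackboard.
; AttackPlayer sphere-traces ahead, playing the attack montage and applying damage on a player hit.
; Hand-built patrol, chase and attack logic remains disconnected, and Tick prints health for debugging.
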(event `self.ReceiveBeginPlay`
  (set `self.Health` (`self.Max Health`)))

(event `self.ReceiveAnyDamage`
  (params (Damage :type "Float (single-precision)") (DamageType :type "DamageType Object Reference") (InstigatedBy :type "Controller Object Reference") (DamageCauser :type "Actor Object Reference"))
  (if (not (`self.IsDeath`))
    (set `self.Health` (- (`self.Health`) Damage))
    (if (<= (`self.Health`) 0)
      (set `self.IsDeath` true)
      (`PrimitiveComponent.SetSimulatePhysics` (`self.Mesh`) true)
      (`|SpawnActorFromClass` "/Game/Agate/finalProject_Sukma_Ciremai/blueprint/Collectible/BP_Ammunition.BP_Ammunition_C" (`KismetMathLibrary.MakeTransform` (`self.K2_GetActorLocation`)) "Undefined" "MultiplyWithRoot" null null)
      (`KismetSystemLibrary.Delay` 3.0)
      (`self.K2_DestroyActor`))))

(event `self.ReceiveTick`
  (params (DeltaSeconds :type "Float (single-precision)"))
  (`KismetSystemLibrary.PrintString` (`KismetStringLibrary.Concat_StrStr` "Enemy Health: " (`KismetStringLibrary.Conv_IntToString` (`self.Health`))) true true (struct :`G` 0.66 :`B` 1.0 :`A` 1.0) 0.0001))

(event `self.PawnSensing.OnSeePawn`
  (params (Pawn :type "Pawn Object Reference"))
  (cast `/Game/Agate/finalProject_Sukma_Ciremai/blueprint/Player/BP_Player` Pawn)
  (`BlackboardComponent.SetValueAsBool` (`AIBlueprintHelperLibrary.GetBlackboard` (`AIBlueprintHelperLibrary.GetAIController` self)) "hasSeenPlayer?" true))

(event `AttackPlayer`
  (bind _returnvalue (`self.K2_GetActorLocation`))
  (bind (_outhit _returnvalue_2) (`KismetSystemLibrary.SphereTraceSingleForObjects` :`Start` _returnvalue :`End` (+ _returnvalue (* (`KismetMathLibrary.GetForwardVector` (`self.K2_GetActorRotation`)) 250.0)) :`Radius` 120.0 :`ObjectTypes` (`|MakeArray` "ObjectTypeQuery3" :!type "EObjectTypeQuery Enum") :`DrawDebugType` "ForDuration"))
  (if _returnvalue_2
    (bind (_bblockinghit _binitialoverlap _time _distance _location _impactpoint _normal _impactnormal _physmat _hitactor) (`GameplayStatics.BreakHitResult` _outhit))
    (cast `/Game/Agate/finalProject_Sukma_Ciremai/blueprint/Player/BP_Player` _hitactor)
    (`self.PlayAnimMontage` "/Game/Agate/Custom_Asset/Enemy/Kuntilanak/Animation/AM_Attack.AM_Attack")
    (`GameplayStatics.ApplyDamage` _hitactor 15.0)))

(event `Patrol`
  ;[1 1 1 1 30] State bikin Manual dari Materi Kursus (attack blm work)
)

(event `ChasePlayer`
  (params (Player :type "Pawn Object Reference"))
  ;[1 1 1 1 30] State bikin Manual dari Materi Kursus (attack blm work)
)

(fn `UserConstructionScript`)