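; BP_EnemySpawner is an actor that spawns enemies at its own location and rotation, either all at once or in timed batches.
; SpawnEnemy loops down a count, spawning one actor per step and adjusting for collisions but always spawning.
; BatchSpawnEnemy calls SpawnEnemy, decrements the batch count, waits out an interval with a Delay and wires back to repeat until no batches remain.
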(event `SpawnEnemy`
  (params (SpawnEnemyCount :type Integer))
  (set `self.SpawnEnemyCount` SpawnEnemyCount)
  (while (> (`self.SpawnEnemyCount`) 0)
    (`|SpawnActorFromClass` "/Game/Agate/finalProject_Sukma_Ciremai/blueprint/Enemy/BP_Enemy.BP_Enemy_C" (`KismetMathLibrary.MakeTransform` (`self.K2_GetActorLocation`) (`self.K2_GetActorRotation`)) "AdjustIfPossibleButAlwaysSpawn" "MultiplyWithRoot" null null)
    (set `self.SpawnEnemyCount` (- (`self.SpawnEnemyCount`) 1))))

(event `BatchSpawnEnemy`
  (params (BatchCount :type Integer) (SpawnEnemyCountPerBatch :type Integer) (Interval :type "Float (double-precision)"))
  (set `self.BatchCount` BatchCount)
  (`self.SpawnEnemy` SpawnEnemyCountPerBatch :!label _label)
  (set `self.BatchCount` (- (`self.BatchCount`) 1))
  (`KismetSystemLibrary.Delay` Interval)
  (if (> (`self.BatchCount`) 0)
    (goto _label)))

(fn `UserConstructionScript`)